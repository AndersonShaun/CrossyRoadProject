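; BP_Car is a car actor that drives continuously along the world X axis.
; Tick scales ForwardSpeed by delta time and passes it to MoveCar, which applies a swept world offset.
; DestroyCar removes the actor and RandomizeCar sets the car mesh with no mesh specified, though neither is called here.
; TriggerZone overlap events are empty, leaving leftover quiz logic that changes speed for BP_Chicken disconnected.
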(event `self.ReceiveTick`
  (params (DeltaSeconds :type "Float (single-precision)"))
  (`self.MoveCar` (* DeltaSeconds (`self.ForwardSpeed`))))

(event `self.TriggerZone.OnComponentBeginOverlap`
  (params (OverlappedComponent :type "PrimitiveComponent Object Reference") (OtherActor :type "Actor Object Reference") (OtherComp :type "PrimitiveComponent Object Reference") (OtherBodyIndex :type Integer) (bFromSweep :type Boolean) (SweepResult :type "HitResult Structure (by ref)"))
  ;[1 1 1] Just for CarStop quiz
)

(event `self.TriggerZone.OnComponentEndOverlap`
  (params (OverlappedComponent :type "PrimitiveComponent Object Reference") (OtherActor :type "Actor Object Reference") (OtherComp :type "PrimitiveComponent Object Reference") (OtherBodyIndex :type Integer))
  ;[1 1 1] Just for CarStop quiz
)

(fn `DestroyCar`
  (`self.K2_DestroyActor`))

(fn `MoveCar`
  (params (Speed :type "Float (double-precision)"))
  (`self.K2_AddActorWorldOffset` (`KismetMathLibrary.MakeVector` Speed) true))

(fn `RandomizeCar`
  (`StaticMeshComponent.SetStaticMesh` (`self.CarMesh`) null))

(fn `UserConstructionScript`)