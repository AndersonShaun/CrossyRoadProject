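; BP_Lane is a lane actor in a chicken crossing game that spawns cars and scores the player's progress.
; Its score zone increments the chicken's score, asks LaneSpawner for another lane, and flags a new level at every multiple of 50.
; Unless Lane is 1, delayed BeginPlay and Tick logic spawns cars, which CarDestroyer removes at the end.
; Another zone destroys the lane when the chicken enters, taking its remaining cars with it.
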(event `self.ScoreZone.OnComponentBeginOverlap`
  (params (OverlappedComponent :type "PrimitiveComponent Object Reference") (OtherActor :type "Actor Object Reference") (OtherComp :type "PrimitiveComponent Object Reference") (OtherBodyIndex :type Integer) (bFromSweep :type Boolean) (SweepResult :type "HitResult Structure (by ref)"))
  (bind _asbp_chicken (cast `/Game/Blueprints/BP_Chicken` OtherActor))
  ;[1 1 1] Increment the player's score
  (bind _result (`/Engine/EditorBlueprintResources/StandardMacros.IncrementInt` (`/Game/Blueprints/BP_Chicken.Score` _asbp_chicken))
    (:`  `
      ;[1 1 1] Check whether to increase the lane size based on score
      (`/Engine/EditorBlueprintResources/StandardMacros.CompareInt` (mod _result 50)
        (:`>`
          _)
        (:`==`
          ;[1 1 1] Set NextLevel flag to increase number of lanes
          (bind _result_2 (`/Engine/EditorBlueprintResources/StandardMacros.IncrementInt` (`/Game/Blueprints/BP_Chicken.CurrentLevel` _asbp_chicken))
            (:`  `
              (set `/Game/Blueprints/BP_Chicken.CurrentLevel` _result_2 _asbp_chicken)
              (set `/Game/Blueprints/BP_Chicken.NextLevel` true _asbp_chicken)))))
      (`/Game/Blueprints/BP_LaneSpawner.SpawnLaneAtSpawnLocation` (`self.LaneSpawner`) 0))))

(event `self.DestroyLaneZone.OnComponentBeginOverlap`
  (params (OverlappedComponent :type "PrimitiveComponent Object Reference") (OtherActor :type "Actor Object Reference") (OtherComp :type "PrimitiveComponent Object Reference") (OtherBodyIndex :type Integer) (bFromSweep :type Boolean) (SweepResult :type "HitResult Structure (by ref)"))
  (cast `/Game/Blueprints/BP_Chicken` OtherActor)
  (`self.K2_DestroyActor`))

(event `self.CarDestroyer.OnComponentBeginOverlap`
  (params (OverlappedComponent :type "PrimitiveComponent Object Reference") (OtherActor :type "Actor Object Reference") (OtherComp :type "PrimitiveComponent Object Reference") (OtherBodyIndex :type Integer) (bFromSweep :type Boolean) (SweepResult :type "HitResult Structure (by ref)"))
  (bind _asbp_car (cast `/Game/Blueprints/BP_Car` OtherActor))
  (`KismetArrayLibrary.Array_Remove` (`self.CarArray`))
  (`/Game/Blueprints/BP_Car.DestroyCar` _asbp_car))

(event `self.ReceiveBeginPlay`
  (`KismetSystemLibrary.Delay` 0.2)
  (`KismetSystemLibrary.PrintText` (`|FormatText` "Lane:{Lane}" (`self.Lane`)))
  (`/Engine/EditorBlueprintResources/StandardMacros.CompareInt` (`self.Lane`) 1
    (:`>`
      (bind _returnvalue (`|SpawnActorFromClass` "/Game/Blueprints/BP_Car.BP_Car_C" (`KismetMathLibrary.MakeTransform` (`SceneComponent.K2_GetComponentLocation` (`self.CarSpawner`)) (struct :`Yaw` 90.0)) "Undefined" "OverrideRootScale" null null :!label _label))
      (`KismetArrayLibrary.Array_Add` (`self.CarArray`) _returnvalue))
    (:`==`
      (`KismetSystemLibrary.PrintText` (`KismetTextLibrary.Conv_IntToText` (`self.Lane`))))
    (:`<`
      (goto _label))))

(event `self.ReceiveTick`
  (params (DeltaSeconds :type "Float (single-precision)"))
  (`KismetSystemLibrary.Delay` 0.2)
  (`/Engine/EditorBlueprintResources/StandardMacros.CompareInt` (`self.Lane`) 1
    (:`>`
      _)
    (:`<`
      _))
  (`KismetSystemLibrary.Delay` 2.0)
  (bind _returnvalue (`|SpawnActorFromClass` "/Game/Blueprints/BP_Car.BP_Car_C" (`KismetMathLibrary.MakeTransform` (`SceneComponent.K2_GetComponentLocation` (`self.CarSpawner`)) (struct :`Yaw` 90.0)) "Undefined" "OverrideRootScale" null null))
  (`KismetArrayLibrary.Array_Add` (`self.CarArray`) _returnvalue))

(event `self.ReceiveDestroyed`
  (for _array_element (`self.CarArray`)
    (`self.K2_DestroyActor` _array_element)))

(fn `UserConstructionScript`)