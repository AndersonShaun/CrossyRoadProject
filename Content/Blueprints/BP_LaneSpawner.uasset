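; Procedural lane spawner for a Crossy Road-style game that builds a grass start area and the first lanes ahead, and spawns an eagle above the chicken.
; SetLaneType picks short runs of road, grass, water or railroad, never repeating the previous type.
; SpawnLaneChunk chains lanes through NextPos, sets meshes with an unmarked last road lane, and adds obstacles or crossings.
; InitLaneVars randomises traffic, flags water and occasionally places coins.
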(event `self.ReceiveBeginPlay`
  (`KismetSystemLibrary.Delay` 0.5)
  (bind _returnvalue (`GameplayStatics.GetActorOfClass` "/Game/Blueprints/BP_Chicken.BP_Chicken_C"))
  (bind (_returnvalue_location _returnvalue_rotation _returnvalue_scale) (`KismetMathLibrary.BreakTransform` (`self.GetTransform` _returnvalue)))
  (bind _returnvalue_2 (`|SpawnActorFromClass` "/Game/Blueprints/SpecialEvent/BP_Eagle.BP_Eagle_C" (`KismetMathLibrary.MakeTransform` (+ (0.0 0.0 1000.0) _returnvalue_location) _returnvalue_rotation _returnvalue_scale) "Undefined" "OverrideRootScale" null null))
  (set `self.EagleRef` _returnvalue_2)
  (`self.SpawnInitialLane`))

(fn `InitLaneVars`
  (params (NewLane :type "/Game/Blueprints/BP_Lane Object Reference"))
  (locals (NewLocalVar :type "Vector Structure" :default (0.0 0.0 0.0)))
  (bind _newestlane (`self.NewestLane`))
  (bind _newestlane_2 (`self.NewestLane`))
  (bind _newestlane_3 (`self.NewestLane`))
  (bind (_currentpos_x _currentpos_y) (`KismetMathLibrary.BreakVector` (`/Game/Blueprints/BP_Lane.CurrentPos` _newestlane_3)))
  (set `/Game/Blueprints/BP_Lane.EagleRef` (`self.EagleRef`) NewLane)
  (bind _output_get (set `self.NewestLane` NewLane))
  (set `/Game/Blueprints/BP_Lane.LaneSpawner` self _output_get)
  (set `/Game/Blueprints/BP_Lane.CurrentPos` (`self.CurrentLaneLocation`) _output_get)
  (if (`self.IsSpawnArea`)
    (set `/Game/Blueprints/BP_Lane.IsWater` false (`self.NewestLane`))
    (`KismetSystemLibrary.PrintString` "Ignore this lane")
    (bind _output_get_2 (set `/Game/Blueprints/BP_Lane.AlreadySteppedOn` true (`self.NewestLane`)))
    (`KismetSystemLibrary.PrintText` (`|FormatText` "Spawn: AlreadySteppedOn:{bool}" _output_get_2))
    (set `/Game/Blueprints/BP_Lane.IsWater` false _newestlane_2 :!label _label)
    (else
      (set `/Game/Blueprints/BP_Lane.Direction` (`KismetMathLibrary.Conv_IntToBool` (`KismetMathLibrary.RandomIntegerInRange` 0 1)) _newestlane)
      ;[1 1 1] Set all the variables for the lane
      (set `/Game/Blueprints/BP_Lane.CarSpeed` (`KismetMathLibrary.RandomIntegerInRange` 100 500) _newestlane)
      (set `/Game/Blueprints/BP_Lane.SpawnDelay` (`KismetMathLibrary.RandomFloatInRange` 0.2 1.0) _newestlane_2)
      (bind _output_get_3 (set `self.LaneType` (`self.LaneType`)))
      (`/Engine/EditorBlueprintResources/StandardMacros.CompareInt` _output_get_3 2
        (:`>`
          (goto _label))
        (:`==`
          (set `/Game/Blueprints/BP_Lane.IsWater` true _newestlane_2))
        (:`<`
          (goto _label)))))
  (set `/Game/Blueprints/BP_Lane.Lane` (`self.LaneType`) _newestlane_3)
  (set `/Game/Blueprints/BP_Lane.NextPos` (`KismetMathLibrary.MakeVector` 0.0 (+ _currentpos_y 120.0)) _newestlane_3)
  (set `/Game/Blueprints/BP_Lane.Boundary` (`SceneComponent.K2_GetComponentLocation` (`/Game/Blueprints/BP_Lane.BoundaryBottom` (`self.NewestLane`))) (`self.NewestLane`))
  (`/Engine/EditorBlueprintResources/StandardMacros.CompareInt` (`KismetMathLibrary.RandomIntegerInRange` 0 20) 19
    (:`>`
      (bind _returnvalue (`|SpawnActorFromClass` "/Game/Blueprints/BP_Coin.BP_Coin_C" (`KismetMathLibrary.MakeTransform` (`SceneComponent.K2_GetComponentLocation` (`/Game/Blueprints/BP_Lane.CoinSpawn1` (`self.NewestLane`)))) "Undefined" "OverrideRootScale" null null :!label _label_2))
      (set `/Game/Blueprints/BP_Lane.Coin` _returnvalue (`self.NewestLane`)))
    (:`==`
      (goto _label_2))
    (:`<`
      _))
  (`self.InitLaneWidth`))

(fn `InitLaneWidth`
  (bind _newestlane (`self.NewestLane`))
  (bind _newestlane_2 (`self.NewestLane`))
  (bind _newestlane_3 (`self.NewestLane`))
  (bind (_currentpos_x _currentpos_y) (`KismetMathLibrary.BreakVector` (`/Game/Blueprints/BP_Lane.CurrentPos` _newestlane_3)))
  (bind (_currentpos_x_2 _currentpos_y_2) (`KismetMathLibrary.BreakVector` (`/Game/Blueprints/BP_Lane.CurrentPos` _newestlane)))
  (bind (_currentpos_x_3 _currentpos_y_3) (`KismetMathLibrary.BreakVector` (`/Game/Blueprints/BP_Lane.CurrentPos` _newestlane_2)))
  (if (`self.IsSpawnArea`)
    (`SceneComponent.K2_SetWorldLocation` (`Actor.RootComponent` _newestlane) (`KismetMathLibrary.MakeVector` 0.0 _currentpos_y_2) false false)
    (else
      ;[1 1 1] Set the DestroyLaneZone and NextLaneSpawnPoint
      (`SceneComponent.K2_SetWorldLocation` (`/Game/Blueprints/BP_Lane.DestroyLaneZone` _newestlane_2) (`KismetMathLibrary.MakeVector` 0.0 (+ _currentpos_y_3 720.0)) false false)
      (`SceneComponent.K2_SetWorldLocation` (`Actor.RootComponent` _newestlane_3) (`KismetMathLibrary.MakeVector` 0.0 _currentpos_y) false false))))

(fn `SetLaneType`
  (params (SpawnLocation :type "Vector Structure"))
  (bind (_currentlanelocation_x _currentlanelocation_y) (`KismetMathLibrary.BreakVector` (`self.CurrentLaneLocation`)))
  (bind _lanetype (`self.LaneType`))
  (if (`self.IsSpawnArea`)
    (`self.SpawnLaneChunk` (`KismetMathLibrary.MakeVector` 0.0 SpawnLocation_Y))
    (else
      ;[1 1 1] When Num of Lanes reaches 0, determine the next type of lane to spawn
      (`/Engine/EditorBlueprintResources/StandardMacros.CompareInt` (`self.NumOfLanes`)
        (:`>`
          _)
        (:`==`
          (set `self.NumOfLanes` (`KismetMathLibrary.RandomIntegerInRange` 1 3))
          ;[1 1 1] Don't spawn another chunk of lanes that was the previous type. Ex: Don't spawn another grass chunk if the previous chunk was grass.
          (while (== (`self.PrevType`) (`self.LaneType`))
            ;[1 1 1] Set the type of the next chunk
            (set `self.LaneType` (`KismetMathLibrary.RandomIntegerInRange` 0 3)))
          ;[1 1 1] Set the type of the previous chunk
          (set `self.PrevType` _lanetype)))
      (`/Engine/EditorBlueprintResources/StandardMacros.CompareInt` _lanetype
        (:`>`
          _)
        (:`==`
          ;[1 1 1] Set Bool flag to true if lane is type road
          (set `self.IsRoadType` true)))
      (`self.SpawnLaneChunk` (`KismetMathLibrary.MakeVector` 0.0 _currentlanelocation_y)))))

(fn `SpawnInitialLane`
  (locals (SpawnGrass :type Boolean))
  (bind (_currentlanelocation_x _currentlanelocation_y) (`KismetMathLibrary.BreakVector` (`self.CurrentLaneLocation`)))
  ;[1 1 1] Render Distance
  (for _ (range 9)
    ;[1 1 1] Check if any lanes exist
    (`/Engine/EditorBlueprintResources/StandardMacros.IsValid` (`self.NewestLane`)
      (:`Is Valid`
        (set `self.IsSpawnArea` false)
        ;[1 1 1] Spawn lanes away from player
        (`self.SpawnLaneAtSpawnLocation` 0))
      (:`Is Not Valid`
        ;[1 1 1] Create the inital spawn area
        (for _ (range 8)
          ;[1 1 1] Set each spawn lane to grass
          (set `self.LaneType` 1)
          ;[1 1 1] Initial grass lanes under player
          (`self.SetLaneType` (`KismetMathLibrary.MakeVector` 0.0 _currentlanelocation_y)))))))

(fn `SpawnLaneAtSpawnLocation`
  (params (LaneWidth :type Integer))
  (bind (_currentlanelocation_x _currentlanelocation_y) (`KismetMathLibrary.BreakVector` (`self.CurrentLaneLocation`)))
  ;[1 1 1] Get the next lane spawn location and spawn a lane there
  (`self.SetLaneType` (`KismetMathLibrary.MakeVector` 0.0 _currentlanelocation_y)))

(fn `SpawnLaneChunk`
  (params (Location :type "Vector Structure"))
  (bind _newestlane (`self.NewestLane`))
  (bind _newestlane_2 (`self.NewestLane`))
  (bind _returnvalue (select `int` (`self.LaneType`) :`0` "/Game/Assets/Crossy/Meshes/road_line.road_line" :`1` "/Game/Assets/Crossy/Meshes/grass.grass" :`2` "/Game/Assets/Crossy/Meshes/water.water" :`3` "/Game/Assets/Crossy/Meshes/railroad_3d.railroad_3d" :!type "StaticMesh Object Reference"))
  (bind _returnvalue_2 (`|SpawnActorFromClass` "/Game/Blueprints/BP_Lane.BP_Lane_C" (`KismetMathLibrary.MakeTransform` (`KismetMathLibrary.MakeVector` 0.0 Location_Y)) "Undefined" "OverrideRootScale" null null))
  (`self.InitLaneVars` _returnvalue_2)
  ;[1 1 1] Determine whether the lane is a road
  (if (`self.IsRoadType`)
    ;[1 1 1] If the lane chunk type is road, set the meshes to marked roads until the last lane of the chunk(Num of Lanes = 1).
    (`/Engine/EditorBlueprintResources/StandardMacros.CompareInt` (`self.NumOfLanes`) 1
      (:`>`
        (`StaticMeshComponent.SetStaticMesh` (`StaticMeshActor.StaticMeshComponent` _newestlane) _returnvalue :!label _label)
        (`StaticMeshComponent.SetStaticMesh` (`/Game/Blueprints/BP_Lane.MeshLeft` _newestlane) _returnvalue)
        (`StaticMeshComponent.SetStaticMesh` (`/Game/Blueprints/BP_Lane.MeshRight` _newestlane) _returnvalue))
      (:`==`
        ;[1 1 1] Since it is the last lane of the road chunk type, set the last lane of the chunk to be an unmarked road and set the flag to false
        (`StaticMeshComponent.SetStaticMesh` (`StaticMeshActor.StaticMeshComponent` _newestlane_2) "/Game/Assets/Crossy/Meshes/road.road")
        (`StaticMeshComponent.SetStaticMesh` (`/Game/Blueprints/BP_Lane.MeshLeft` _newestlane_2) "/Game/Assets/Crossy/Meshes/road.road")
        (`StaticMeshComponent.SetStaticMesh` (`/Game/Blueprints/BP_Lane.MeshRight` _newestlane_2) "/Game/Assets/Crossy/Meshes/road.road")
        (set `self.IsRoadType` false)))
    (else
      (goto _label)))
  ;[1 1 1] Set the location of the next lane to be the current location
  (set `self.CurrentLaneLocation` (`/Game/Blueprints/BP_Lane.NextPos` (`self.NewestLane`)))
  ;[1 1 1] Spawn RRCrossing Object if lane type is railroad
  (`/Engine/EditorBlueprintResources/StandardMacros.CompareInt` (`self.LaneType`) 3
    (:`>`
      _)
    (:`==`
      (bind _returnvalue_3 (`|SpawnActorFromClass` "/Game/Blueprints/BP_RRCrossing.BP_RRCrossing_C" (`KismetMathLibrary.MakeTransform` (`SceneComponent.K2_GetComponentLocation` (`/Game/Blueprints/BP_Lane.RRCrossing` (`self.NewestLane`))) (struct :`Yaw` 90.0)) "Undefined" "OverrideRootScale" null null))
      (set `/Game/Blueprints/BP_Lane.RRCrossingObj` _returnvalue_3 (`self.NewestLane`)))
    (:`<`
      (`/Engine/EditorBlueprintResources/StandardMacros.CompareInt` (`self.LaneType`) 1
        (:`>`
          _)
        (:`==`
          (bind _returnvalue_4 (`|SpawnActorFromClass` "/Game/Blueprints/BP_Obstacle.BP_Obstacle_C" (`KismetMathLibrary.MakeTransform` (`SceneComponent.K2_GetComponentLocation` (`/Game/Blueprints/BP_Lane.TreeSpawnLeft` (`self.NewestLane`)))) "Undefined" "OverrideRootScale" null null))
          (`KismetArrayLibrary.Array_Add` (`/Game/Blueprints/BP_Lane.ObstacleArray` (`self.NewestLane`)) _returnvalue_4)
          (bind _returnvalue_5 (`|SpawnActorFromClass` "/Game/Blueprints/BP_Obstacle.BP_Obstacle_C" (`KismetMathLibrary.MakeTransform` (`SceneComponent.K2_GetComponentLocation` (`/Game/Blueprints/BP_Lane.TreeSpawnRight` (`self.NewestLane`)))) "Undefined" "OverrideRootScale" null null))
          (`KismetArrayLibrary.Array_Add` (`/Game/Blueprints/BP_Lane.ObstacleArray` (`self.NewestLane`)) _returnvalue_5))
        (:`<`
          _))))
  (if (not (`self.IsSpawnArea`))
    ;[1 1 1] Decrement Num of Lanes by 1
    (`/Engine/EditorBlueprintResources/StandardMacros.DecrementInt` (`self.NumOfLanes`))))

(fn `UserConstructionScript`)