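; BP_Railroad_Sign is a railroad sign actor that flashes its left and right lights.
; Tick decrements a Count variable and, when it reaches zero, inverts the visibility of LightRight and LightLeft and resets the counter.
; The flash interval is counted in frames, so its speed depends on frame rate.
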(event `self.ReceiveBeginPlay`)

(event `self.ReceiveTick`
  (params (DeltaSeconds :type "Float (single-precision)"))
  (bind _result (`/Engine/EditorBlueprintResources/StandardMacros.DecrementInt` (`self.Count`))
    (:`  `
      (if (== _result 0)
        (`SceneComponent.SetVisibility` (`self.Light Right`) (not (`SceneComponent.IsVisible` (`self.Light Right`))) false)
        (`SceneComponent.SetVisibility` (`self.Light Left`) (not (`SceneComponent.IsVisible` (`self.Light Left`))) false)
        (set `self.Count` 20)))))

(fn `UserConstructionScript`)