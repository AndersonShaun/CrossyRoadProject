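; Railroad crossing that runs a repeating train event once RailRoadSpawned starts its timer.
; Randomly delayed timers chain PrepareTrain, CallTrain and EndTrainEvent: lower the arm, ring the bell and park a BP_Car train at a random lane end, launch it, then reset.
; Tick flashes the warning lights during the event, while timelines animate the arm and fade out the bell.
; Destroying the crossing also destroys its current train.
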(event `self.ReceiveTick`
  (params (DeltaSeconds :type "Float (single-precision)"))
  (if (`self.TrainEventActive`)
    (bind _output_get (set `self.TimeSinceToggle` (+ (`self.TimeSinceToggle`) DeltaSeconds)))
    (if (>= _output_get 0.5)
      (`SceneComponent.ToggleVisibility` (`self.LeftLight`) false)
      (`SceneComponent.ToggleVisibility` (`self.RightLight`) false)
      (set `self.TimeSinceToggle` 0.0))))

(event `RailRoadSpawned`
  (`KismetSystemLibrary.K2_SetTimer` null "PrepareTrain" (`KismetMathLibrary.RandomFloatInRange` (`self.MinTrainDelay`) (`self.MaxTrainDelay`))))

(event `LowerArm`
  (bind (_direction _armrotation) (`Timeline|LoweringArm` :!via `PlayFromStart`)
    (:`Update`
      (`SceneComponent.K2_SetRelativeRotation` (`self.railroad_arm`) (`KismetMathLibrary.MakeRotator` (.x _armrotation)) false false))))

(event `StopRRBell`
  (bind (_direction _alpha _armrotation) (`Timeline|Timeline` :!via `PlayFromStart`)
    (:`Update`
      (`AudioComponent.SetVolumeMultiplier` (`self.RailRoadBell`) _alpha)
      (`SceneComponent.K2_SetRelativeRotation` (`self.railroad_arm`) (`KismetMathLibrary.MakeRotator` (.x _armrotation)) false false))
    (:`Finished`
      (`ActorComponent.K2_DestroyComponent` (`self.RailRoadBell`)))))

(event `self.ReceiveDestroyed`
  (bind _train (`self.Train`))
  (`/Engine/EditorBlueprintResources/StandardMacros.IsValid` _train
    (:`Is Valid`
      (`self.K2_DestroyActor` _train))))

(fn `CallTrain`
  (bind _train (`self.Train`))
  (`/Game/Blueprints/BP_Car.ActivateTrainSound` _train)
  (`/Game/Blueprints/BP_Car.SetSpeed` _train (`self.TrainDirection`) 3000 0)
  (`KismetSystemLibrary.K2_SetTimer` null "EndTrainEvent" (`KismetMathLibrary.RandomFloatInRange` (`self.MinTrainDelay`) (`self.MaxTrainDelay`))))

(fn `EndTrainEvent`
  (`SceneComponent.SetVisibility` (`self.LeftLight`) false true)
  (`self.StopRRBell`)
  (set `self.TrainEventActive` false)
  (`KismetSystemLibrary.K2_SetTimer` null "PrepareTrain" (`KismetMathLibrary.RandomFloatInRange` 4.0 10.0)))

(fn `PrepareTrain`
  (bind _returnvalue (`KismetMathLibrary.RandomBool`))
  (set `self.TrainEventActive` true)
  (`self.LowerArm`)
  (bind _returnvalue_2 (`GameplayStatics.SpawnSoundAttached` "/Game/Assets/Crossy/Sounds/RR_Bell_Cue.RR_Bell_Cue" (`self.RRCrossingSign`) "None" (0.0 0.0 0.0) (struct) "KeepRelativeOffset" false 1.0 1.0 0.0 null null))
  (set `self.RailRoadBell` _returnvalue_2)
  (if (`KismetMathLibrary.RandomBool`)
    (`SceneComponent.ToggleVisibility` (`self.LeftLight`) false)
    (else
      (`SceneComponent.ToggleVisibility` (`self.RightLight`) false)))
  (bind _output_get (set `self.TrainDirection` _returnvalue))
  (if _output_get
    (bind _returnvalue_3 (`|SpawnActorFromClass` "/Game/Blueprints/BP_Car.BP_Car_C" (`KismetMathLibrary.MakeTransform` (`SceneComponent.K2_GetComponentLocation` (`/Game/Blueprints/BP_Lane.CarSpawnerLeft` (`self.Lane`))) (struct :`Yaw` -90.0)) "Undefined" "OverrideRootScale" null null))
    (bind _output_get_2 (set `self.Train` _returnvalue_3))
    (`/Game/Blueprints/BP_Lane.SetMesh` (`self.Lane`) _output_get_2)
    (`/Game/Blueprints/BP_Car.SetSpeed` _output_get_2 _returnvalue 4 3)
    (`SceneComponent.K2_AddWorldOffset` (`/Game/Blueprints/BP_Car.CarMesh` _output_get_2) (0.0 0.0 40.0) false false)
    (`/Game/Blueprints/BP_Car.ChangeCollisionSize` _output_get_2 3)
    (set `/Game/Blueprints/BP_Car.ForwardSpeed` 0.0 _output_get_2)
    (else
      (bind _returnvalue_4 (`|SpawnActorFromClass` "/Game/Blueprints/BP_Car.BP_Car_C" (`KismetMathLibrary.MakeTransform` (`SceneComponent.K2_GetComponentLocation` (`/Game/Blueprints/BP_Lane.CarSpawnerRight` (`self.Lane`))) (struct :`Yaw` 90.0)) "Undefined" "OverrideRootScale" null null))
      (bind _output_get_3 (set `self.Train` _returnvalue_4))
      (`/Game/Blueprints/BP_Lane.SetMesh` (`self.Lane`) _output_get_3)
      (`/Game/Blueprints/BP_Car.SetSpeed` _output_get_3 (not _returnvalue) 4 3)
      (`SceneComponent.K2_AddWorldOffset` (`/Game/Blueprints/BP_Car.CarMesh` _returnvalue_4) (0.0 0.0 40.0) false false)
      (`/Game/Blueprints/BP_Car.ChangeCollisionSize` _output_get_3 3)
      (set `/Game/Blueprints/BP_Car.ForwardSpeed` 0.0 _output_get_3)))
  (`KismetSystemLibrary.K2_SetTimer` null "CallTrain" (`KismetMathLibrary.RandomFloatInRange` (`self.MinTrainDelay`) (`self.MaxTrainDelay`))))

(fn `UserConstructionScript`)