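; Obstacle spawner that creates moving car obstacles at the newest lane's left or right spawn point.
; SpawnCar randomly picks a side and rotation, spawns a BP_MovingObstacle, gives it a random speed negated when Reverse is set, and randomly assigns one of two car meshes.
; SpawnOnLeft is an unfinished typed left-side spawn, and the event graph is empty, so nothing here triggers spawning.
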(fn `Spawn Car`
  (locals (SpawnLocation :type "Vector Structure") (SpawnRotation :type "Rotator Structure") (Reverse :type Boolean))
  (bind _returnvalue (`KismetMathLibrary.RandomIntegerInRange` 100 1000))
  ;[1 1 1] Comment
  (switch `int` (`KismetMathLibrary.RandomInteger` 2)
    (:`0`
      (set `local.SpawnLocation` (`SceneComponent.K2_GetComponentLocation` (`/Game/Blueprints/BP_Lane.ObstacleSpawnLeft` (`self.NewestLane`))))
      (set `local.SpawnRotation` (struct)))
    (:`1`
      (set `local.Reverse` false)
      (set `local.SpawnLocation` (`SceneComponent.K2_GetComponentLocation` (`/Game/Blueprints/BP_Lane.ObstacleSpawnRight` (`self.NewestLane`))))
      (set `local.SpawnRotation` (struct :`Yaw` 180.0))))
  (bind _returnvalue_2 (`|SpawnActorFromClass` "/Game/Blueprints/BP_MovingObstacle.BP_MovingObstacle_C" (`KismetMathLibrary.MakeTransform` (`local.SpawnLocation`) (`local.SpawnRotation`)) "Undefined" "OverrideRootScale" null null))
  (if (`local.Reverse`)
    (set `/Game/Blueprints/BP_MovingObstacle.MaxSpeed` (* _returnvalue -1) _returnvalue_2)
    (else
      (set `/Game/Blueprints/BP_MovingObstacle.MaxSpeed` _returnvalue _returnvalue_2)))
  (`StaticMeshComponent.SetStaticMesh` (`StaticMeshActor.StaticMeshComponent` _returnvalue_2) (select `int` (`KismetMathLibrary.RandomInteger` 2) :`0` "/Game/Mesh/car.car" :`1` "/Game/Mesh/car_convertible_topdown.car_convertible_topdown" :!type "StaticMesh Object Reference")))

(fn `SpawnOnLeft`
  (params (Type :type "/Game/Blueprints/ObstacleEnums Enum" :default "NewEnumerator0"))
  (returns (CreatedObstacle :type "/Game/Blueprints/BP_MovingObstacle Object Reference"))
  (`|SpawnActorFromClass` "/Game/Blueprints/BP_MovingObstacle.BP_MovingObstacle_C" (`KismetMathLibrary.MakeTransform` (`SceneComponent.K2_GetComponentLocation` (`/Game/Blueprints/BP_Lane.ObstacleSpawnLeft` (`self.NewestLane`)))) "Undefined" "OverrideRootScale" null null)
  (switch `/Game/Blueprints/ObstacleEnums` Type))

(fn `UserConstructionScript`)