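; Eagle hazard that flies along its local X axis and kills BP_Chicken on contact.
; BeginPlay caches the chicken, scales and rotates the eagle, then Tick moves it with a swept offset.
; KillZone overlap moves the chicken mesh onto DeadMesh, so the eagle appears to carry it, then calls Die.
; Dive teleports it near the chicken with a shriek, but its timer is disconnected and the score events are empty.
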(event `self.ReceiveBeginPlay`
  (bind _returnvalue (`GameplayStatics.GetActorOfClass` "/Game/Blueprints/BP_Chicken.BP_Chicken_C"))
  (set `self.ChickenRef` _returnvalue)
  (`self.SetActorRelativeScale3D` (0.75 0.75 0.75))
  (`self.K2_SetActorRotation` (struct :`Yaw` 180.0)))

(event `self.ReceiveTick`
  (params (DeltaSeconds :type "Float (single-precision)"))
  (`self.K2_AddActorLocalOffset` (`KismetMathLibrary.MakeVector` (* DeltaSeconds (`self.MovementSpeed`))) true))

(event `ScoreHasNotIncreased`)

(event `ScoreHasIncreased`)

(event `self.Kill Zone.OnComponentBeginOverlap`
  (params (OverlappedComponent :type "PrimitiveComponent Object Reference") (OtherActor :type "Actor Object Reference") (OtherComp :type "PrimitiveComponent Object Reference") (OtherBodyIndex :type Integer) (bFromSweep :type Boolean) (SweepResult :type "HitResult Structure (by ref)"))
  (bind _asbp_chicken (cast `/Game/Blueprints/BP_Chicken` OtherActor))
  (`SkeletalMeshComponent.SetSkeletalMeshAsset` (`Character.Mesh` _asbp_chicken) null)
  (`SkeletalMeshComponent.SetSkeletalMeshAsset` (`self.DeadMesh`) "/Game/Assets/Crossy/chicken.chicken")
  (`/Game/Blueprints/BP_Chicken.Die` _asbp_chicken))

(fn `CirclePlayer`)

(fn `Dive`
  (bind (_returnvalue_x _returnvalue_y _returnvalue_z) (`KismetMathLibrary.BreakVector` (`self.K2_GetActorLocation` (`self.ChickenRef`))))
  (`self.K2_SetActorLocation` (`KismetMathLibrary.MakeVector` (+ _returnvalue_x -1000.0) _returnvalue_y (+ _returnvalue_z 50.0)))
  (`GameplayStatics.SpawnSoundAttached` "/Game/Assets/Crossy/Sounds/Eagle_Shriek_Cue.Eagle_Shriek_Cue" (`self.DefaultSceneRoot`) "None" (0.0 0.0 0.0) (struct) "KeepRelativeOffset" false 1.0 1.0 0.0 null null))

(fn `UserConstructionScript`)